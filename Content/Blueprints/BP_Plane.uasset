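; BP_Plane is a player-controlled plane that rotates and fires rockets through Enhanced Input actions.
; IA_Rotate applies local roll from the X axis and pitch from the Y axis, scaled by RotateSpeed and frame delta time.
; IA_Fire spawns a MyRocket at the Arrow component's world transform.
; The IA_Boost event and construction script are empty, and the graph contains no forward-movement logic.
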(event Input|EnhancedActionEvents|EnhancedInputActionIA_Rotate
  (params (ActionValue :type Vector%202D%20Structure) (ElapsedSeconds :type Float%20%28double-precision%29) (TriggeredSeconds :type Float%20%28double-precision%29) (InputAction :type Input%20Action%20Object%20Reference :default "/Game/Inputs/IA_Rotate.IA_Rotate"))
  (Transformation|AddActorLocalRotation (Math|Rotator|MakeRotator (* (.x ActionValue) (Utilities|Time|GetWorldDeltaSeconds) (Variables|Default|GetRotateSpeed)) 0.0 0.0) false false)
  (Transformation|AddActorLocalRotation (Math|Rotator|MakeRotator 0.0 (* (.y ActionValue) (Utilities|Time|GetWorldDeltaSeconds) (Variables|Default|GetRotateSpeed)) 0.0) false false))

(event Input|EnhancedActionEvents|EnhancedInputActionIA_Fire
  (params (ActionValue :type Boolean) (ElapsedSeconds :type Float%20%28double-precision%29) (TriggeredSeconds :type Float%20%28double-precision%29) (InputAction :type Input%20Action%20Object%20Reference :default "/Game/Inputs/IA_Fire.IA_Fire"))
  (Game|SpawnActorfromClass "/Script/UE20260415.MyRocket" (Transformation|GetWorldTransform (Variables|Default|GetArrow)) "Undefined" "MultiplyWithRoot" 0 0))

(event Input|EnhancedActionEvents|EnhancedInputActionIA_Boost
  (params (ActionValue :type Boolean) (ElapsedSeconds :type Float%20%28double-precision%29) (TriggeredSeconds :type Float%20%28double-precision%29) (InputAction :type Input%20Action%20Object%20Reference :default "/Game/Inputs/IA_Boost.IA_Boost")))

(fn ConstructionScript)